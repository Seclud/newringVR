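; A seat actor that lets the VR pawn sit down and stand up.
; SitArea overlaps toggle CanSit for the VR pawn, and show or hide a Widget and Cube through visibility and material opacity for any actor.
; Sit snaps the player pawn onto the seat by attachment and lowers its camera.
; Stand detaches the pawn and teleports it to the SitLocation and SitRotation stored on it.
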(event `/Game/BluePrints/InteractBP.Stand`
  (if (stale `/Game/BluePrints/InteractBP.Sit` _output_get)
    (`self.K2_DetachFromActor` (stale `/Game/BluePrints/InteractBP.Sit` _asvrpawn) "KeepRelative" "KeepRelative" "KeepRelative")
    (`self.K2_SetActorLocationAndRotation` (stale `/Game/BluePrints/InteractBP.Sit` _asvrpawn) (`/Game/VRTemplate/Blueprints/VRPawn.SitLocation` (stale `/Game/BluePrints/InteractBP.Sit` _asvrpawn)) (`/Game/VRTemplate/Blueprints/VRPawn.SitRotation` (stale `/Game/BluePrints/InteractBP.Sit` _asvrpawn)) false true)
    (set `self.IsSitting` false)))

(event `/Game/BluePrints/InteractBP.Sit`
  (bind _asvrpawn (cast `/Game/VRTemplate/Blueprints/VRPawn` (`GameplayStatics.GetPlayerPawn` 0)))
  (if (`self.CanSit`)
    (bind _returnvalue (`self.K2_AttachToActor` _asvrpawn self "None" "SnapToTarget" "KeepRelative" "KeepRelative" true))
    (if _returnvalue
      (`/Game/VRTemplate/Blueprints/VRPawn.Move Camera Lower to Sit` _asvrpawn)
      (bind _output_get (set `self.IsSitting` true)))))

(event `self.SitArea.OnComponentBeginOverlap`
  (params (OverlappedComponent :type "PrimitiveComponent Object Reference") (OtherActor :type "Actor Object Reference") (OtherComp :type "PrimitiveComponent Object Reference") (OtherBodyIndex :type Integer) (bFromSweep :type Boolean) (SweepResult :type "HitResult Structure (by ref)"))
  (`|ExecutionSequence`
    (:`then_0`
      (cast `/Game/VRTemplate/Blueprints/VRPawn` OtherActor)
      (if true
        (set `self.CanSit` true)))
    (:`then_1`
      (bind _returnvalue (`PrimitiveComponent.CreateDynamicMaterialInstance` (`self.Cube`) 0 null "None"))
      (bind _output_get (set `self.dynamic material instnace` _returnvalue))
      (`MaterialInstanceDynamic.SetScalarParameterValue` _output_get "Opacity" 1.0)
      (`KismetSystemLibrary.PrintString` "Hello"))
    (:`then_2`
      (`SceneComponent.SetVisibility` (`self.Widget`) true false))))

(event `self.SitArea.OnComponentEndOverlap`
  (params (OverlappedComponent :type "PrimitiveComponent Object Reference") (OtherActor :type "Actor Object Reference") (OtherComp :type "PrimitiveComponent Object Reference") (OtherBodyIndex :type Integer))
  (`|ExecutionSequence`
    (:`then_0`
      (bind _returnvalue (`PrimitiveComponent.CreateDynamicMaterialInstance` (`self.Cube`) 0 null "None"))
      (bind _output_get (set `self.dynamic material instnace` _returnvalue))
      (`MaterialInstanceDynamic.SetScalarParameterValue` _output_get "Opacity" 0.0)
      (`KismetSystemLibrary.PrintString` "Goodbye"))
    (:`then_1`
      (cast `/Game/VRTemplate/Blueprints/VRPawn` OtherActor)
      (if true
        (set `self.CanSit` false)))
    (:`then_2`
      (`SceneComponent.SetVisibility` (`self.Widget`) false false))))

(fn `UserConstructionScript`)