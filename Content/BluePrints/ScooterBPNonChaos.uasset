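; A drivable VR scooter moved kinematically by offsetting and yawing the actor each tick, with no physics or delta-time scaling.
; Grabbing the lever sets a fixed speed and releasing it stops the scooter.
; Grabbing the steering runs a looping timer that turns it toward the motion controller, mapping its clamped yaw to the steering angle.
; The enter grab toggles riding by aligning and attaching the VR origin, or detaching it at the exit position.
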(event `self.ReceiveTick`
  (params (DeltaSeconds :type "Float (single-precision)"))
  (bind _speed (`self.Speed`))
  ;[0 0 0] Throttling
  (`self.K2_AddActorWorldOffset` (* (`self.GetActorForwardVector`) _speed))
  (`self.K2_AddActorWorldRotation` (`KismetMathLibrary.MakeRotator` 0.0 0.0 (* _speed (`self.SteeringAngle`) (`self.SpeedToRotationFactor`)))))

(event `self.LeverGB.OnGrabbed`
  (params (`Motion Contoller` :type "MotionControllerComponent Object Reference"))
  ;[0 0 0] Throttling
  (set `self.Speed` 5.0))

(event `self.LeverGB.OnDropped`
  ;[0 0 0] Throttling
  (set `self.Speed` 0.0))

(event `self.EnterGB.OnGrabbed`
  (params (`Motion Contoller` :type "MotionControllerComponent Object Reference"))
  (bind (_returnvalue_x _returnvalue_y) (`KismetMathLibrary.BreakVector` (`SceneComponent.K2_GetComponentLocation` (`self.ExitPosition`))))
  ;[0 0 0] Enter The Scooter
  (bind _asvrpawn (cast `/Game/VRTemplate/Blueprints/VRPawn` (`GameplayStatics.GetPlayerPawn` 0)))
  (if (`self.OnScooter`)
    (bind _vrorigin (`/Game/VRTemplate/Blueprints/VRPawn.VROrigin` _asvrpawn))
    (`SceneComponent.K2_SetWorldLocation` _vrorigin (`KismetMathLibrary.MakeVector` _returnvalue_x _returnvalue_y) false false)
    (`HeadMountedDisplayFunctionLibrary.SetTrackingOrigin` "Stage")
    (set `self.OnScooter` false)
    (`SceneComponent.K2_DetachFromComponent` _vrorigin "KeepWorld" "KeepWorld" "KeepWorld" true)
    (else
      (`SceneComponent.K2_AddWorldOffset` _vrorigin (- (`SceneComponent.K2_GetComponentLocation` (`self.HeadPosition`)) (`SceneComponent.K2_GetComponentLocation` (`/Game/VRTemplate/Blueprints/VRPawn.Camera` _asvrpawn))) false false)
      (set `self.OnScooter` true)
      (`SceneComponent.K2_AttachToComponent` _vrorigin (`self.HeadPosition`) "None" "KeepWorld" "KeepWorld" "KeepWorld" true))))

(event `self.SteeringGB.OnGrabbed`
  (params (`Motion Contoller` :type "MotionControllerComponent Object Reference"))
  ;[0 0 0] Steering
  (set `self.SteeringMC` `Motion Contoller`)
  (`KismetSystemLibrary.K2_SetTimerDelegate` (delegate `RotateWheel`) 0.01 true))

(event `RotateWheel`
  (bind _steering (`self.Steering`))
  (bind _steering_2 (`self.Steering`))
  (bind (_relativerotation_roll _relativerotation_pitch _relativerotation_yaw) (`KismetMathLibrary.BreakRotator` (`SceneComponent.RelativeRotation` _steering_2)))
  ;[0 0 0] Steering
  (`SceneComponent.K2_AddLocalRotation` _steering_2 (`KismetMathLibrary.MakeRotator` 0.0 0.0 (* (`KismetMathLibrary.NormalizeAxis` (`KismetMathLibrary.Dot_VectorVector` (`KismetMathLibrary.Conv_RotatorToVector` (`KismetMathLibrary.FindLookAtRotation` (`SceneComponent.K2_GetComponentLocation` _steering) (`SceneComponent.K2_GetComponentLocation` (`self.SteeringMC`)))) (`KismetMathLibrary.GetForwardVector` (`SceneComponent.K2_GetComponentRotation` _steering)))) 50.0)) false false)
  (set `self.SteeringAngle` (`KismetMathLibrary.MapRangeClamped` _relativerotation_yaw -20.0 20.0 1.0 -1.0)))

(event `self.SteeringGB.OnDropped`
  ;[0 0 0] Steering
  (`KismetSystemLibrary.K2_PauseTimer` null "RotateWheel")
  (set `self.SteeringMC` null))

(fn `UserConstructionScript`)